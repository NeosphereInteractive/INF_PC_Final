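; Base ship Blueprint for player, ally and enemy ships, handling the main camera and the zoomed-in weapon view.
; Construction fits four side trigger boxes to the hull bounds for player and ally ships, and strips camera and trigger components from enemies.
; Zooming traces from an arrow to pick the nearest weapon of the active type, blends the view to it and allows index-based cycling.
; Camera input drives the ship camera or the active weapon and its companions.
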(event `self.ReceiveBeginPlay`
  (bind _asplayer_ship_controller_bp (cast `/Game/Blueprints/Controllers/PlayerShipController_BP` (`GameplayStatics.GetPlayerController` 0)))
  (set `self.PlayerShipControllerRef` _asplayer_ship_controller_bp)
  (`KismetSystemLibrary.Delay` 0.5)
  (set `/Game/Blueprints/ShipsAndBirds/ShipParent_BP.MainShipRef` null (`/Game/Blueprints/Controllers/PlayerShipController_BP.MainShip` (`self.PlayerShipControllerRef`))))

(event `CameraAzimuth`
  (params (axisValue :type "Float (double-precision)") (cameraState :type "/Game/Blueprints/Enumerations/E_CameraState Enum" :default "NewEnumerator0") (`hasCompanion?` :type Boolean))
  (switch `/Game/Blueprints/Enumerations/E_CameraState` cameraState
    (:`NewEnumerator0`
      (`self.AzimuthMainCamera` axisValue))
    (:`NewEnumerator1`
      (`self.AzimuthWeapon` axisValue `hasCompanion?`))))

(event `CameraElevation`
  (params (axisValue :type "Float (double-precision)") (cameraState :type "/Game/Blueprints/Enumerations/E_CameraState Enum" :default "NewEnumerator0") (`hasCompanion?` :type Boolean))
  (switch `/Game/Blueprints/Enumerations/E_CameraState` cameraState
    (:`NewEnumerator0`
      (`self.ElevateMainCamera` axisValue))
    (:`NewEnumerator1`
      (`self.ElevateWeapon` axisValue `hasCompanion?`))))

(event `SimpleDelay`
  (params (functionName :type String) (delayAmount :type "Float (double-precision)"))
  (`KismetSystemLibrary.K2_SetTimer` null functionName delayAmount))

(event `TurnOnCameraInput`
  (set `/Game/Blueprints/Controllers/PlayerShipController_BP.cameraInputOn?` true (`self.PlayerShipControllerRef`)))

(fn `AddToDistanceTable`
  (params (weapon :type "Actor Object Reference"))
  (`KismetArrayLibrary.Array_Add` (`self.distanceTableTemp`) (`KismetMathLibrary.VSize` (- (`self.K2_GetActorLocation` weapon) (`self.impactPointTemp`)))))

(fn `AzimuthMainCamera`
  (params (axisValue :type "Float (double-precision)"))
  (`SceneComponent.K2_AddWorldRotation` (`self.MainSpringArm`) (`KismetMathLibrary.MakeRotator` 0.0 0.0 (* axisValue (`self.MainCameraAzimuthRate`))) false false))

(fn `AzimuthWeapon`
  (params (axisValue :type "Float (double-precision)") (`hasCompanion?` :type Boolean))
  (if `hasCompanion?`
    (bind _currentactivatedweapon (`self.currentActivatedWeapon`)
      (:`then`
        (`/Game/Blueprints/Weapons/WeaponParent_BP.AzimuthWeapon` _currentactivatedweapon axisValue true)
        (for _array_element (`self.companionsTemp`)
          (`/Game/Blueprints/Weapons/WeaponParent_BP.AzimuthWeapon` _array_element axisValue false)))
      (:`else`))
    (else
      (bind _currentactivatedweapon_2 (`self.currentActivatedWeapon`)
        (:`then`
          (`/Game/Blueprints/Weapons/WeaponParent_BP.AzimuthWeapon` _currentactivatedweapon_2 axisValue false))
        (:`else`)))))

(fn `ElevateMainCamera`
  (params (axisValue :type "Float (double-precision)"))
  (bind (_relativerotation_roll _relativerotation_pitch _relativerotation_yaw) (`KismetMathLibrary.BreakRotator` (`SceneComponent.RelativeRotation` (`self.MainShipCamera`))))
  (`SceneComponent.K2_SetRelativeRotation` (`self.MainShipCamera`) (`KismetMathLibrary.MakeRotator` _relativerotation_roll (`KismetMathLibrary.FClamp` (+ (* axisValue (`self.MainCameraElevationRate`)) _relativerotation_pitch) 0.0 (`self.MaxMainCameraEvelation`)) _relativerotation_yaw) false false))

(fn `ElevateWeapon`
  (params (axisValue :type "Float (double-precision)") (`hasCompanion?` :type Boolean))
  (if `hasCompanion?`
    (bind _currentactivatedweapon (`self.currentActivatedWeapon`)
      (:`then`
        (`/Game/Blueprints/Weapons/WeaponParent_BP.ElevateWeapon` _currentactivatedweapon axisValue false)
        (for _array_element (`self.companionsTemp`)
          (`/Game/Blueprints/Weapons/WeaponParent_BP.ElevateWeapon` _array_element axisValue false)))
      (:`else`))
    (else
      (bind _currentactivatedweapon_2 (`self.currentActivatedWeapon`)
        (:`then`
          (`/Game/Blueprints/Weapons/WeaponParent_BP.ElevateWeapon` _currentactivatedweapon_2 axisValue false))
        (:`else`)))))

(fn `GetClosestWeapon`
  (params (weaponType :type "/Game/Blueprints/Enumerations/E_Weapons Enum" :default "NewEnumerator0") (impactPoint :type "Vector Structure (by ref)"))
  (bind _playershipcontrollerref (`self.PlayerShipControllerRef`))
  (bind (_output_ship _output_aaguns _output_seahawks _output_seakings) (break `/Game/Blueprints/Structures/Struct_ShipWeapons` (`|GetArrayItem` (`/Game/Blueprints/Controllers/PlayerShipController_BP.ShipWeaponsTable` _playershipcontrollerref) (`/Game/Blueprints/Controllers/PlayerShipController_BP.CurrentShipIndex` _playershipcontrollerref))))
  (set `self.impactPointTemp` impactPoint)
  (switch `/Game/Blueprints/Enumerations/E_Weapons` weaponType
    (:`NewEnumerator0`
      (for _array_element _output_aaguns
        (`self.AddToDistanceTable` _array_element))
      (bind _output_get (set `self.currentActivatedWeapon` (`|GetArrayItem` _output_aaguns (`KismetMathLibrary.MinOfFloatArray` (`self.distanceTableTemp`)))))
      (`self.SetHasCompanion` _output_get)
      (`self.MoveToWeapon` _output_get))
    (:`NewEnumerator1`
      (for _array_element_2 _output_seahawks
        (`self.AddToDistanceTable` _array_element_2))
      (bind _output_get_2 (set `self.currentActivatedWeapon` (`|GetArrayItem` _output_seahawks (`KismetMathLibrary.MinOfFloatArray` (`self.distanceTableTemp`)))))
      (`self.SetHasCompanion` _output_get_2)
      (`self.MoveToWeapon` _output_get_2))
    (:`NewEnumerator2`
      (for _array_element_3 _output_seakings
        (`self.AddToDistanceTable` _array_element_3))
      (bind _output_get_3 (set `self.currentActivatedWeapon` (`|GetArrayItem` _output_seakings (`KismetMathLibrary.MinOfFloatArray` (`self.distanceTableTemp`)))))
      (`self.SetHasCompanion` _output_get_3)
      (`self.MoveToWeapon` _output_get_3))))

(fn `GetDistanceToShipCentre`
  (returns (Distance :type "Float (double-precision)"))
  (bind _shipbody (`self.ShipBody`))
  (return (`KismetMathLibrary.VSize` (- (`SceneComponent.GetSocketLocation` _shipbody "CentrePoint") (`SceneComponent.GetSocketLocation` _shipbody "BottomPoint")))))

(fn `GetWeaponWithIndex`
  (for _array_element (`self.currentActivatedWeaponTable`)
    (if (== (`/Game/Blueprints/Weapons/WeaponParent_BP.WeaponIndex` _array_element) (`self.moveToWeaponWithIndex`))
      (set `self.currentActivatedWeapon` _array_element)
      (break))))

(fn `JumpToAdjacentWeapon`
  (params (direction :type Integer))
  (bind _weaponindex (`/Game/Blueprints/Weapons/WeaponParent_BP.WeaponIndex` (`self.currentActivatedWeapon`)))
  (switch `int` direction
    (:`-1`
      (if (== (`/Game/Blueprints/Weapons/WeaponParent_BP.WeaponIndex` (`self.currentActivatedWeapon`)) 1)
        (set `self.moveToWeaponWithIndex` (`BlueprintMapLibrary.Map_Find` (`self.AllWeaponsInfo`) (`self.WeaponType`)))
        (else
          (set `self.moveToWeaponWithIndex` (- _weaponindex 1)))))
    (:`1`
      (if (>= (`/Game/Blueprints/Weapons/WeaponParent_BP.WeaponIndex` (`self.currentActivatedWeapon`)) (`BlueprintMapLibrary.Map_Find` (`self.AllWeaponsInfo`) (`self.WeaponType`)))
        (set `self.moveToWeaponWithIndex` 1)
        (else
          (set `self.moveToWeaponWithIndex` (+ _weaponindex 1))))))
  (`self.GetWeaponWithIndex`)
  (`self.MoveToWeapon` (`self.currentActivatedWeapon`)))

(fn `MoveToWeapon`
  (params (ownerRef :type "Actor Object Reference (by ref)"))
  (`PlayerController.SetViewTargetWithBlend` (`self.PlayerShipControllerRef`) ownerRef 1.0 "VTBlend_Cubic" 0.0 false)
  (`KismetSystemLibrary.K2_SetTimer` null "TurnOnCameraInput" 1.1))

(fn `ResetZoomVariables`
  (set `self.currentActivatedWeapon` null)
  (set `self.impactPointTemp` (0.0 0.0 0.0))
  (`KismetArrayLibrary.Array_Clear` (`self.distanceTableTemp`))
  (`KismetArrayLibrary.Array_Clear` (`self.companionsTemp`)))

(fn `SetActivatedWeaponType`
  (params (activatedWeaponType :type "/Game/Blueprints/Enumerations/E_Weapons Enum" :default "NewEnumerator0") (weaponsArray :type "Array of /Game/Blueprints/Weapons/WeaponParent_BP Object Reference (by ref)") (autoSelectWeapon :type Boolean))
  (set `self.WeaponType` activatedWeaponType)
  (bind _output_get (set `self.currentActivatedWeaponTable` weaponsArray))
  (if (and (== (`KismetArrayLibrary.Array_Length` _output_get) 1) autoSelectWeapon)
    (set `/Game/Blueprints/Controllers/PlayerShipController_BP.cameraInputOn?` false (`self.PlayerShipControllerRef`))
    (bind _output_get_2 (set `self.currentActivatedWeapon` (`|GetArrayItem` (`self.currentActivatedWeaponTable`))))
    (`self.MoveToWeapon` _output_get_2)
    (set `/Game/Blueprints/Controllers/PlayerShipController_BP.CurrentCameraState` "NewEnumerator1" (`self.PlayerShipControllerRef`))
    (elif (and (> (`KismetArrayLibrary.Array_Length` (`self.currentActivatedWeaponTable`)) 1) autoSelectWeapon (`|EnumEquality` (`/Game/Blueprints/Controllers/PlayerShipController_BP.CurrentCameraState` (`self.PlayerShipControllerRef`)) "NewEnumerator1"))
      (`self.ZoomOutIntoMainView`))))

(fn `SetBoxHeight`
  (params (distance :type "Float (double-precision)"))
  (for _array_element (`self.WeaponsTriggerTable`)
    (bind (_returnvalue_x _returnvalue_y _returnvalue_z) (`KismetMathLibrary.BreakVector` (`SceneComponent.K2_GetComponentLocation` _array_element)))
    (`SceneComponent.K2_SetWorldLocation` _array_element (+ (`KismetMathLibrary.MakeVector` _returnvalue_x _returnvalue_y (+ _returnvalue_z distance)) (`SceneComponent.K2_GetComponentLocation` (`self.ShipBody`))) false false)))

(fn `SetBoxPositionAndScale`
  (bind _shipsize_x (`KismetMathLibrary.BreakVector` (`self.ShipSize`)))
  (bind (_shipsize_x_2 _shipsize_y) (`KismetMathLibrary.BreakVector` (`self.ShipSize`)))
  (bind _shipsize_x_3 (`KismetMathLibrary.BreakVector` (`self.ShipSize`)))
  (bind (_shipsize_x_4 _shipsize_y_2) (`KismetMathLibrary.BreakVector` (`self.ShipSize`)))
  (`|ExecutionSequence`
    (:`then_0`
      (`SceneComponent.K2_SetWorldLocation` (`self.WeaponTrigger_Left`) (`KismetMathLibrary.MakeVector` 0.0 (* _shipsize_y_2 -1.0)) false false)
      (`BoxComponent.SetBoxExtent` (`self.WeaponTrigger_Left`) (`self.ShipSize`) true)
      (`SceneComponent.SetWorldScale3D` (`self.WeaponTrigger_Left`) (1.0 0.1 1.0)))
    (:`then_1`
      (`SceneComponent.K2_SetWorldLocation` (`self.WeaponTrigger_Right`) (`KismetMathLibrary.MakeVector` 0.0 _shipsize_y) false false)
      (`BoxComponent.SetBoxExtent` (`self.WeaponTrigger_Right`) (`self.ShipSize`) true)
      (`SceneComponent.SetWorldScale3D` (`self.WeaponTrigger_Right`) (1.0 0.1 1.0)))
    (:`then_2`
      (`SceneComponent.K2_SetWorldLocation` (`self.WeaponTrigger_Front`) (`KismetMathLibrary.MakeVector` _shipsize_x_3) false false)
      (`BoxComponent.SetBoxExtent` (`self.WeaponTrigger_Front`) (`self.ShipSize`) true)
      (`SceneComponent.SetWorldScale3D` (`self.WeaponTrigger_Front`) (0.02 1.0 1.0)))
    (:`then_3`
      (`SceneComponent.K2_SetWorldLocation` (`self.WeaponTrigger_Back`) (`KismetMathLibrary.MakeVector` (* _shipsize_x -1.0)) false false)
      (`BoxComponent.SetBoxExtent` (`self.WeaponTrigger_Back`) (`self.ShipSize`) true)
      (`SceneComponent.SetWorldScale3D` (`self.WeaponTrigger_Back`) (0.02 1.0 1.0)))))

(fn `UserConstructionScript`
  (bind _array (`|MakeArray` (`self.WeaponTrigger_Left`) (`self.WeaponTrigger_Right`) (`self.WeaponTrigger_Front`) (`self.WeaponTrigger_Back`)))
  (switch `/Game/Blueprints/Enumerations/E_ShipType` (`self.ShipType`)
    (:`NewEnumerator0`
      (set `self.WeaponsTriggerTable` (`|MakeArray` (`self.WeaponTrigger_Left`) (`self.WeaponTrigger_Right`) (`self.WeaponTrigger_Front`) (`self.WeaponTrigger_Back`)) :!label _label)
      (set `self.ShipSize` (`.BoxExtent` (`KismetSystemLibrary.GetComponentBounds` (`self.ShipBody`))))
      (`self.SetBoxPositionAndScale`)
      (bind _distance (`self.GetDistanceToShipCentre`))
      (`self.SetBoxHeight` _distance))
    (:`NewEnumerator1`
      (goto _label))
    (:`NewEnumerator2`
      (`ActorComponent.K2_DestroyComponent` (`self.MainSpringArm`))
      (`ActorComponent.K2_DestroyComponent` (`self.MainShipCamera`))
      (`ActorComponent.K2_DestroyComponent` (`self.RaycastArrow`))
      (for _array_element _array
        (`ActorComponent.K2_DestroyComponent` _array_element))
      (`KismetArrayLibrary.Array_Clear` _array))))

(fn `ZoomIntoWeapon`
  (locals (rayImpactPointTemp :type "Vector Structure" :default (0.0 0.0 0.0)))
  (bind _raycastarrow (`self.RaycastArrow`))
  (bind _returnvalue (`SceneComponent.K2_GetComponentLocation` _raycastarrow))
  (set `/Game/Blueprints/Controllers/PlayerShipController_BP.CurrentCameraState` "NewEnumerator1" (`self.PlayerShipControllerRef`))
  (bind (_outhit _returnvalue_2) (`KismetSystemLibrary.LineTraceSingle` :`Start` _returnvalue :`End` (+ _returnvalue (* (`KismetMathLibrary.GetForwardVector` (`SceneComponent.K2_GetComponentRotation` _raycastarrow)) 10000.0)) :`TraceChannel` "TraceTypeQuery3" :`bIgnoreSelf` false :`DrawTime` 15.0))
  (if _returnvalue_2
    (`self.GetClosestWeapon` (`self.WeaponType`) (`.ImpactPoint` (`GameplayStatics.BreakHitResult` _outhit)))))

(fn `ZoomOutIntoMainView`
  (`self.ResetZoomVariables`)
  (`PlayerController.SetViewTargetWithBlend` (`self.PlayerShipControllerRef`) self 1.0 "VTBlend_Cubic" 0.0 false)
  (set `/Game/Blueprints/Controllers/PlayerShipController_BP.CurrentCameraState` "NewEnumerator0" (`self.PlayerShipControllerRef`)))