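; Veer_BP is a player ship driven by physics forces on its Box component, with automatic forward thrust and player steering.
; BeginPlay waits a few seconds, then enables Tick, which pushes along the Box's forward vector at PushForcePos.
; The MoveRight axis applies sideways force at SteerPos along its right vector.
; Both forces scale with mass, but only thrust scales with frame time.
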(event `self.ReceiveBeginPlay`
  (`parent.ReceiveBeginPlay`)
  (`KismetSystemLibrary.Delay` 5.0)
  (`self.SetActorTickEnabled` true)
  (`KismetSystemLibrary.PrintString` "Move Ship now!"))

(event `self.ReceiveTick`
  (params (DeltaSeconds :type "Float (single-precision)"))
  (bind _box (`self.Box`))
  (`parent.ReceiveTick` DeltaSeconds)
  (`PrimitiveComponent.AddForceAtLocation` (`self.Box`) (* (`KismetMathLibrary.GetForwardVector` (`SceneComponent.K2_GetComponentRotation` _box)) (* (`PrimitiveComponent.GetMass` _box) 459136.0 DeltaSeconds)) (`SceneComponent.K2_GetComponentLocation` (`self.PushForcePos`)) "None"))

(event `InputAxis|MoveRight`
  (params (AxisValue :type "Float (single-precision)"))
  (bind _steerpos (`self.SteerPos`))
  (`PrimitiveComponent.AddForceAtLocation` (`self.Box`) (* (`KismetMathLibrary.GetRightVector` (`SceneComponent.K2_GetComponentRotation` _steerpos)) (* (* (`PrimitiveComponent.GetMass` (`self.Box`)) 200.0) AxisValue)) (`SceneComponent.K2_GetComponentLocation` _steerpos) "None"))

(fn `UserConstructionScript`
  (`parent.UserConstructionScript`))