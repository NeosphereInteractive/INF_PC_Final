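; Player controller for the ship that handles camera, weapon selection and weapon zoom input.
; On BeginPlay it builds a table of each eligible ship's AA guns, Seahawks and Seakings from child actors, then finds the player's ship.
; Input switches to available weapon types, zooms, and jumps between adjacent weapons, forwarding actions to that ship.
; It also pairs AA guns as companions when the dot product of their forward vectors is roughly non-negative.
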(event `self.ReceiveBeginPlay`
  (bind (_output_ship _output_aaguns) (break `/Game/Blueprints/Structures/Struct_ShipWeapons` (`|GetArrayItem` (`self.ShipWeaponsTable`) (`self.CurrentShipIndex`))))
  (bind _outactors (`GameplayStatics.GetAllActorsOfClass` "/Game/Blueprints/ShipsAndBirds/ShipParent_BP.ShipParent_BP_C"))
  (`self.SetupShipWeaponsTable` _outactors)
  (`KismetSystemLibrary.Delay` 0.2)
  (`self.SetDefaultWeapon` false)
  (`self.GetCompanionWeapons` _output_aaguns))

(event `InputAxis|CameraAzimuth`
  (params (AxisValue :type "Float (single-precision)"))
  ;[0 1 0] Ship and Weapon Camera manipulation
  (if (`self.cameraInputOn?`)
    (`/Game/Blueprints/ShipsAndBirds/ShipParent_BP.CameraAzimuth` (`self.MainShip`) AxisValue (`self.CurrentCameraState`) (`self.HasCompanion?`))))

(event `InputAction|SelectAAGun`
  (params (Key :type "Key Structure"))
  (bind (_output_ship _output_aaguns) (break `/Game/Blueprints/Structures/Struct_ShipWeapons` (`|GetArrayItem` (`self.ShipWeaponsTable`) (`self.CurrentShipIndex`))))
  ;[0 1 0] Weapon Selection
  (:`Pressed`
    (if (`|EnumInequality` (`/Game/Blueprints/ShipsAndBirds/ShipParent_BP.WeaponType` (`self.MainShip`)) "NewEnumerator0")
      (bind _shouldswitch_ (`self.CanSwitchToWeapon?` "NewEnumerator0"))
      (if _shouldswitch_
        (`/Game/Blueprints/ShipsAndBirds/ShipParent_BP.SetActivatedWeaponType` (`self.MainShip`) "NewEnumerator0" _output_aaguns true)
        (`KismetSystemLibrary.PrintString` "Anti-Aircraft Gun Selected!" true true (struct :`G` 0.66 :`B` 1.0 :`A` 1.0) 5.0)))))

(event `InputAxis|CameraElevation`
  (params (AxisValue :type "Float (single-precision)"))
  ;[0 1 0] Ship and Weapon Camera manipulation
  (if (`self.cameraInputOn?`)
    (`/Game/Blueprints/ShipsAndBirds/ShipParent_BP.CameraElevation` (`self.MainShip`) AxisValue (`self.CurrentCameraState`) (`self.HasCompanion?`))))

(event `InputAction|SelectSeahawk`
  (params (Key :type "Key Structure"))
  (bind (_output_ship _output_aaguns _output_seahawks) (break `/Game/Blueprints/Structures/Struct_ShipWeapons` (`|GetArrayItem` (`self.ShipWeaponsTable`) (`self.CurrentShipIndex`))))
  ;[0 1 0] Weapon Selection
  (:`Pressed`
    (if (`|EnumInequality` (`/Game/Blueprints/ShipsAndBirds/ShipParent_BP.WeaponType` (`self.MainShip`)) "NewEnumerator1")
      (bind _shouldswitch_ (`self.CanSwitchToWeapon?` "NewEnumerator1"))
      (if _shouldswitch_
        (`/Game/Blueprints/ShipsAndBirds/ShipParent_BP.SetActivatedWeaponType` (`self.MainShip`) "NewEnumerator1" _output_seahawks true)
        (`KismetSystemLibrary.PrintString` "Seahawk Selected!" true true (struct :`G` 0.66 :`B` 1.0 :`A` 1.0) 5.0)))))

(event `InputAction|SelectSeaking`
  (params (Key :type "Key Structure"))
  (bind (_output_ship _output_aaguns _output_seahawks _output_seakings) (break `/Game/Blueprints/Structures/Struct_ShipWeapons` (`|GetArrayItem` (`self.ShipWeaponsTable`) (`self.CurrentShipIndex`))))
  ;[0 1 0] Weapon Selection
  (:`Pressed`
    (if (`|EnumInequality` (`/Game/Blueprints/ShipsAndBirds/ShipParent_BP.WeaponType` (`self.MainShip`)) "NewEnumerator2")
      (bind _shouldswitch_ (`self.CanSwitchToWeapon?` "NewEnumerator2"))
      (if _shouldswitch_
        (`/Game/Blueprints/ShipsAndBirds/ShipParent_BP.SetActivatedWeaponType` (`self.MainShip`) "NewEnumerator2" _output_seakings true)
        (`KismetSystemLibrary.PrintString` "Seaking Selected!" true true (struct :`G` 0.66 :`B` 1.0 :`A` 1.0) 5.0)))))

(event `InputAction|ZoomIn`
  (params (Key :type "Key Structure"))
  ;[0 1 0] Zoom in/out to/from weapon!
  (:`Pressed`
    (if (`|EnumEquality` (`self.CurrentCameraState`) "NewEnumerator0")
      (`/Game/Blueprints/ShipsAndBirds/ShipParent_BP.ZoomIntoWeapon` (`self.MainShip`)))))

(event `InputAction|MoveToWeaponLeft`
  (params (Key :type "Key Structure"))
  (:`Pressed`
    (if (and (`|EnumEquality` (`self.CurrentCameraState`) "NewEnumerator1") (`self.canJumpToWeapon?`))
      (`/Game/Blueprints/ShipsAndBirds/ShipParent_BP.JumpToAdjacentWeapon` (`self.MainShip`) -1))))

(event `InputAction|ZoomOut`
  (params (Key :type "Key Structure"))
  ;[0 1 0] Zoom in/out to/from weapon!
  (:`Pressed`
    (if (`|EnumEquality` (`self.CurrentCameraState`) "NewEnumerator1")
      (`/Game/Blueprints/ShipsAndBirds/ShipParent_BP.ZoomOutIntoMainView` (`self.MainShip`)))))

(event `InputAction|MoveToWeaponRight`
  (params (Key :type "Key Structure"))
  (:`Pressed`
    (if (and (`|EnumEquality` (`self.CurrentCameraState`) "NewEnumerator1") (`self.canJumpToWeapon?`))
      (`/Game/Blueprints/ShipsAndBirds/ShipParent_BP.JumpToAdjacentWeapon` (`self.MainShip`) 1))))

(event `GetWeaponsFromShip`
  (params (ship :type "/Game/Blueprints/ShipsAndBirds/ShipParent_BP Object Reference") (index :type Integer))
  (bind _allweaponsinfo (`/Game/Blueprints/ShipsAndBirds/ShipParent_BP.AllWeaponsInfo` (`self.tempShipRef`)))
  (bind _output_get (set `self.tempShipRef` ship))
  (for _array_element (`self.GetAllChildActors` _output_get true)
    (bind _asweapon_parent_bp (cast `/Game/Blueprints/Weapons/WeaponParent_BP` _array_element))
    (switch `/Game/Blueprints/Enumerations/E_Weapons` (`/Game/Blueprints/Weapons/WeaponParent_BP.WeaponType` _asweapon_parent_bp)
      (:`NewEnumerator0`
        (bind _asaagun_bp (cast `/Game/Blueprints/Weapons/AAGun_BP` _asweapon_parent_bp))
        (bind _returnvalue (`KismetArrayLibrary.Array_AddUnique` (`self.AAGuns`) _asaagun_bp))
        (bind _result (`/Engine/EditorBlueprintResources/StandardMacros.IncrementInt` _returnvalue)
          (:`  `
            (`BlueprintMapLibrary.Map_Add` _allweaponsinfo "" _result))))
      (:`NewEnumerator1`
        (bind _asseahawk_bp (cast `/Game/Blueprints/Weapons/Seahawk_BP` _asweapon_parent_bp))
        (bind _returnvalue_2 (`KismetArrayLibrary.Array_AddUnique` (`self.Seahawks`) _asseahawk_bp))
        (bind _result_2 (`/Engine/EditorBlueprintResources/StandardMacros.IncrementInt` _returnvalue_2)
          (:`  `
            (`BlueprintMapLibrary.Map_Add` _allweaponsinfo "NewEnumerator1" _result_2))))
      (:`NewEnumerator2`
        (bind _asseaking_bp (cast `/Game/Blueprints/Weapons/Seaking_BP` _asweapon_parent_bp))
        (bind _returnvalue_3 (`KismetArrayLibrary.Array_AddUnique` (`self.Seakings`) _asseaking_bp))
        (bind _result_3 (`/Engine/EditorBlueprintResources/StandardMacros.IncrementInt` _returnvalue_3)
          (:`  `
            (`BlueprintMapLibrary.Map_Add` _allweaponsinfo "NewEnumerator2" _result_3))))))
  (`KismetArrayLibrary.Array_AddUnique` (`self.ShipWeaponsTable`) (make `/Game/Blueprints/Structures/Struct_ShipWeapons` (`self.tempShipRef`) (`self.AAGuns`) (`self.Seahawks`) (`self.Seakings`) (`|MakeMap` "NewEnumerator0" :!type "/Game/Blueprints/Enumerations/E_Weapons Enum")))
  (set `self.tempShipRef` null))

(fn `CanSwitchToWeapon?`
  (params (targetWeaponType :type "/Game/Blueprints/Enumerations/E_Weapons Enum" :default "NewEnumerator0"))
  (returns (`shouldSwitch?` :type Boolean))
  (bind _value (`BlueprintMapLibrary.Map_Find` (`/Game/Blueprints/ShipsAndBirds/ShipParent_BP.AllWeaponsInfo` (`self.MainShip`)) targetWeaponType))
  (if (> _value 0)
    (if (> _value 1)
      (set `self.canJumpToWeapon?` true)
      (else
        (set `self.canJumpToWeapon?` false)))
    (return true)
    (else
      (set `self.canJumpToWeapon?` false)
      (return false))))

(fn `GetCompanionWeapons`
  (params (weaponsArray :type "Array of /Game/Blueprints/Weapons/WeaponParent_BP Object Reference (by ref)"))
  (locals (weaponsArrayTemp :type "Array of /Game/Blueprints/Weapons/WeaponParent_BP Object Reference"))
  (bind _weaponsarraytemp (`local.weaponsArrayTemp`))
  (if (> (`KismetArrayLibrary.Array_Length` weaponsArray) 0)
    (bind _output_get (set `local.weaponsArrayTemp` weaponsArray))
    (bind _returnvalue (- (`KismetArrayLibrary.Array_Length` _output_get) 1))
    (for _index (range (+ _returnvalue 1))
      (for _index_2 (range (+ _returnvalue 1))
        (bind _output (`|GetArrayItem` _weaponsarraytemp _index_2))
        (bind _output_2 (`|GetArrayItem` _weaponsarraytemp _index))
        (if (!= _output _output_2)
          (if (>= (`KismetMathLibrary.Dot_VectorVector` (`self.GetActorForwardVector` _output) (`self.GetActorForwardVector` _output_2)) -0.01)
            (`KismetArrayLibrary.Array_AddUnique` (`/Game/Blueprints/Weapons/WeaponParent_BP.Companions` _output) _output_2)
            (`KismetArrayLibrary.Array_AddUnique` (`/Game/Blueprints/Weapons/WeaponParent_BP.Companions` _output_2) _output)))))))

(fn `GetMainShip`
  (for (_array_element _array_index) (`self.ShipWeaponsTable`)
    (if (== (break `/Game/Blueprints/Structures/Struct_ShipWeapons` _array_element) (`GameplayStatics.GetPlayerPawn` 0))
      (set `self.MainShip` (break `/Game/Blueprints/Structures/Struct_ShipWeapons` _array_element))
      (set `self.CurrentShipIndex` _array_index)
      (break))))

(fn `SetDefaultWeapon`
  (params (`autoSelectWeapon?` :type Boolean))
  (bind _mainship (`self.MainShip`))
  (bind (_output_ship _output_aaguns _output_seahawks _output_seakings) (break `/Game/Blueprints/Structures/Struct_ShipWeapons` (`|GetArrayItem` (`self.ShipWeaponsTable`) (`self.CurrentShipIndex`))))
  (switch `/Game/Blueprints/Enumerations/E_Weapons` (`/Game/Blueprints/ShipsAndBirds/ShipParent_BP.WeaponType` (`self.MainShip`))
    (:`NewEnumerator0`
      (`/Game/Blueprints/ShipsAndBirds/ShipParent_BP.SetActivatedWeaponType` _mainship "NewEnumerator0" _output_aaguns `autoSelectWeapon?`)
      (`self.CanSwitchToWeapon?` "NewEnumerator0"))
    (:`NewEnumerator1`
      (`/Game/Blueprints/ShipsAndBirds/ShipParent_BP.SetActivatedWeaponType` _mainship "NewEnumerator1" _output_seahawks `autoSelectWeapon?`)
      (`self.CanSwitchToWeapon?` "NewEnumerator1"))
    (:`NewEnumerator2`
      (`/Game/Blueprints/ShipsAndBirds/ShipParent_BP.SetActivatedWeaponType` _mainship "NewEnumerator2" _output_seakings `autoSelectWeapon?`)
      (`self.CanSwitchToWeapon?` "NewEnumerator2"))))

(fn `SetupShipWeaponsTable`
  (params (AllFriendlyShips :type "Array of /Game/Blueprints/ShipsAndBirds/ShipParent_BP Object Reference (by ref)"))
  (locals (allShipsTableTemp :type "Array of /Game/Blueprints/ShipsAndBirds/ShipParent_BP Object Reference"))
  (if (> (`KismetArrayLibrary.Array_Length` AllFriendlyShips) 0)
    (bind _output_get (set `local.allShipsTableTemp` AllFriendlyShips))
    (for _array_element _output_get
      (if (`|EnumInequality` (`/Game/Blueprints/ShipsAndBirds/ShipParent_BP.ShipType` _array_element) "NewEnumerator2")
        (`self.GetWeaponsFromShip` _array_element)))
    (`self.GetMainShip`)))

(fn `UserConstructionScript`)