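; Parent Blueprint for ship weapons, providing a gun that is aimed by rotating a turret and a barrel.
; Interface events add axis input to turret yaw and barrel pitch, clamped to azimuth and elevation limits.
; When azimuth input is flagged for a companion, a visibility trace runs forward from the gun camera, ignoring the main ship.
; That trace currently only draws debug lines and prints the hit actor's name.
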(event `/Game/Blueprints/Interfaces/BPI_Weapon.AzimuthWeapon`
  (params (axisValue :type "Float (single-precision)") (`ForCompanion?` :type Boolean))
  (bind (_relativerotation_roll _relativerotation_pitch _relativerotation_yaw) (`KismetMathLibrary.BreakRotator` (`SceneComponent.RelativeRotation` (`self.GunTurret`))))
  (`SceneComponent.K2_SetRelativeRotation` (`self.GunTurret`) (`KismetMathLibrary.MakeRotator` 0.0 0.0 (`KismetMathLibrary.FClamp` (+ axisValue _relativerotation_yaw) (`self.minAzimuth`) (`self.maxAzimuth`))) false false)
  (if `ForCompanion?`
    (`self.LineTraceForCompanions`)))

(event `/Game/Blueprints/Interfaces/BPI_Weapon.ElevateWeapon`
  (params (axisValue :type "Float (single-precision)") (`ForCompanion?` :type Boolean))
  (bind (_relativerotation_roll _relativerotation_pitch) (`KismetMathLibrary.BreakRotator` (`SceneComponent.RelativeRotation` (`self.GunBarrel`))))
  (bind (_relativerotation_roll_2 _relativerotation_pitch_2 _relativerotation_yaw) (`KismetMathLibrary.BreakRotator` (`SceneComponent.RelativeRotation` (`self.GunBarrel`))))
  (`SceneComponent.K2_SetRelativeRotation` (`self.GunBarrel`) (`KismetMathLibrary.MakeRotator` _relativerotation_roll_2 (`KismetMathLibrary.FClamp` (+ axisValue _relativerotation_pitch) (`self.minElevation`) (`self.maxElevation`)) _relativerotation_yaw) false false))

(fn `LineTraceForCompanions`
  (bind _guncamera (`self.GunCamera`))
  (bind _returnvalue (`SceneComponent.K2_GetComponentLocation` _guncamera))
  (bind _outhit (`KismetSystemLibrary.LineTraceSingle` _returnvalue (+ _returnvalue (* (`KismetMathLibrary.GetForwardVector` (`SceneComponent.K2_GetComponentRotation` _guncamera)) 10000.0)) "TraceTypeQuery1" false (`|MakeArray` (`self.MainShipRef`) :!type "Actor Object Reference") "ForDuration" true (struct :`R` 1.0 :`A` 1.0) (struct :`G` 1.0 :`A` 1.0) 10.0))
  (`KismetSystemLibrary.PrintString` (`KismetSystemLibrary.GetDisplayName` (`.HitActor` (`GameplayStatics.BreakHitResult` _outhit)))))

(fn `UserConstructionScript`
  (`parent.UserConstructionScript`))